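; Game mode for an anime runner game that times the player's run.
; On BeginPlay it adds the time widget to the viewport and starts a timeline that writes its track value into Time every update.
; It also binds to the runner player controller's death delegate, which stops the timer and calls PostMatchTime.
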(event `self.ReceiveBeginPlay`
  (`|ExecutionSequence`
    (:`then_0`
      ;[0.4708 1 0.6808] Add Timer on Screen
      (bind _returnvalue (`|CreateWidget` "/Game/Blueprints/UI/Gameplay/WBP_Time.WBP_Time_C"))
      (`UserWidget.AddToViewport` _returnvalue 0)
      (bind (_direction _newtrack_1) (`Timeline|Timeline_Timer`)
        (:`Update`
          (set `self.Time` _newtrack_1))))
    (:`then_1`
      ;[1 0.3438 0.3438] On Death Event
      (bind _asbp_runner_player_controller (cast `/Game/Blueprints/BP_RunnerPlayerController` (`GameplayStatics.GetPlayerController` 0)))
      (add `RunnerPlayerController.OnDeathDelegate` _asbp_runner_player_controller (delegate `OnDeathDelegate_Event_0`)))))

(event `OnDeathDelegate_Event_0`
  ;[1 0.3438 0.3438] On Death Event
  (`TimelineComponent.Stop` (`self.Timeline_Timer`))
  (`self.PostMatchTime`))

(fn `UserConstructionScript`)