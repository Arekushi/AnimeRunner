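; BP_Platform03 is a platform variant that tells its parent logic which block obstacles sit above each of its floors.
; On BeginPlay it runs the parent's logic, then calls AddObstaclesAbove to link Floor02 to Block03 and Block02, and Floor01 to Block01.
; Floors are passed as child actor components, and the construction script only calls the parent's.
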(event `self.ReceiveBeginPlay`
  (`parent.ReceiveBeginPlay`)
  (`|ExecutionSequence`
    (:`then_0`
      (`self.AddObstaclesAbove` (`self.Floor_02`) (`|MakeArray` (`self.Block_03`) (`self.Block_02`))))
    (:`then_1`
      (`self.AddObstaclesAbove` (`self.Floor_01`) (`|MakeArray` (`self.Block_01`))))))

(fn `UserConstructionScript`
  (`parent.UserConstructionScript`))