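; BP_RunnerPlayer is a 2D player character Blueprint that keeps its sprite's flipbook in sync with movement state and facing.
; On BeginPlay it binds to movement-status and animation-direction delegates, both of which call UpdateFlipbook.
; UpdateFlipbook uses nested Selects on direction and status to pick an "emi" flipbook, with Run reusing walk animations.
; Left and Right share side-view flipbooks and additionally call Flip.
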(event `OnAnimationDirectionUpdateDelegate_Event_0`
  (`self.UpdateFlipbook` :!label _label))

(event `self.ReceiveBeginPlay`
  (add `self.OnMovementStatusUpdateDelegate` (delegate `OnMovementStatusUpdateDelegate_Event_0`))
  (add `self.OnAnimationDirectionUpdateDelegate` (delegate `OnAnimationDirectionUpdateDelegate_Event_0`)))

(event `OnMovementStatusUpdateDelegate_Event_0`
  (goto _label))

(fn `UpdateFlipbook`
  (bind _animationdirection (`self.AnimationDirection`))
  (bind _movementstatus (`self.MovementStatus`))
  (bind _returnvalue (select `ECharacterMovementStatus` _movementstatus :`Stop` "/Game/Flipbooks/Character/FB_emi_x_stop.FB_emi_x_stop" :`Walk` "/Game/Flipbooks/Character/FB_emi_x_walk.FB_emi_x_walk" :`Run` "/Game/Flipbooks/Character/FB_emi_x_walk.FB_emi_x_walk" :`Jump` "/Game/Flipbooks/Character/FB_emi_x_jump.FB_emi_x_jump" :`Fall` "/Game/Flipbooks/Character/FB_emi_x_fall.FB_emi_x_fall" :`Idle` "/Game/Flipbooks/Character/FB_emi_x_idle.FB_emi_x_idle" :!type "PaperFlipbook Object Reference"))
  (`PaperFlipbookComponent.SetFlipbook` (`self.Sprite`) (select `ECharacterAnimationDirection` _animationdirection :`Up` (select `ECharacterMovementStatus` _movementstatus :`Stop` "/Game/Flipbooks/Character/FB_emi_up_stop.FB_emi_up_stop" :`Walk` "/Game/Flipbooks/Character/FB_emi_up_walk.FB_emi_up_walk" :`Run` "/Game/Flipbooks/Character/FB_emi_up_walk.FB_emi_up_walk" :`Jump` "/Game/Flipbooks/Character/FB_emi_up_jump.FB_emi_up_jump" :`Fall` "/Game/Flipbooks/Character/FB_emi_up_fall.FB_emi_up_fall" :`Idle` "/Game/Flipbooks/Character/FB_emi_up_idle.FB_emi_up_idle" :!type "PaperFlipbook Object Reference") :`Down` (select `ECharacterMovementStatus` _movementstatus :`Stop` "/Game/Flipbooks/Character/FB_emi_down_stop.FB_emi_down_stop" :`Walk` "/Game/Flipbooks/Character/FB_emi_down_walk.FB_emi_down_walk" :`Run` "/Game/Flipbooks/Character/FB_emi_down_walk.FB_emi_down_walk" :`Jump` "/Game/Flipbooks/Character/FB_emi_down_jump.FB_emi_down_jump" :`Fall` "/Game/Flipbooks/Character/FB_emi_down_fall.FB_emi_down_fall" :`Idle` "/Game/Flipbooks/Character/FB_emi_down_idle.FB_emi_down_idle" :!type "PaperFlipbook Object Reference") :`Left` _returnvalue :`Right` _returnvalue))
  (if (select `ECharacterAnimationDirection` _animationdirection :`Left` true :`Right` true)
    (`self.Flip`)))

(fn `UserConstructionScript`)