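; Player controller for the runner game that handles the death screen and restart sequence.
; On BeginPlay it binds its Death event to an OnDeath delegate.
; Death fades the camera out and shows the WBP_You_Died widget.
; After a delay it starts a fade back in, removes all widgets and calls RestartGame on BP_AnimeRunner_GameMode.
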(event `self.ReceiveBeginPlay`
  (add `self.OnDeathDelegate` (delegate `Death`)))

(event `Death`
  (`PlayerCameraManager.StartCameraFade` :`self` (`GameplayStatics.GetPlayerCameraManager` 0) :`ToAlpha` 1.0 :`Duration` 1.0 :`bHoldWhenFinished` true)
  (bind _returnvalue (`|CreateWidget` "/Game/Blueprints/UI/Gameplay/WBP_You_Died.WBP_You_Died_C" self))
  (`UserWidget.AddToViewport` _returnvalue 0)
  (`KismetSystemLibrary.Delay` 4.0)
  (`PlayerCameraManager.StartCameraFade` :`self` (`GameplayStatics.GetPlayerCameraManager` 0) :`FromAlpha` 1.0 :`Duration` 2.0 :`bHoldWhenFinished` true)
  (`WidgetLayoutLibrary.RemoveAllWidgets`)
  (bind _asbp_anime_runner_game_mode (cast `/Game/Blueprints/BP_AnimeRunner_GameMode` (`GameplayStatics.GetGameMode`)))
  (`GameMode.RestartGame` _asbp_anime_runner_game_mode))

(fn `UserConstructionScript`)